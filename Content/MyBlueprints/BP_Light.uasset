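; BP_Light is a light fixture that switches to a blinking red emergency light when an Explosion event fires.
; On BeginPlay it binds handlers to the Explosion, Enable and Disable events.
; The explosion handler recolors the mesh and point light, sets intensity, then enters the On state.
; On and Off toggle visibility and material, each calling the other's event after a delay to form an endless, uneven blink.
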(event `self.ReceiveBeginPlay`
  (add `self.Explosion` (delegate `EmergencyLights`))
  (add `self.Disable` (delegate `Off`))
  (add `self.Enable` (delegate `On`)))

(event `Off`
  (`SceneComponent.SetVisibility` (`self.PointLight`) false false)
  (`PrimitiveComponent.SetMaterial` (`self.StaticMeshComponent`) 1 "/Game/Materials/M_Black.M_Black")
  (`KismetSystemLibrary.Delay` 0.6)
  (`self.Enable`))

(event `On`
  (`SceneComponent.SetVisibility` (`self.PointLight`) true false :!label _label)
  (`PrimitiveComponent.SetMaterial` (`self.StaticMeshComponent`) 1 "/Game/Materials/M_Red_Inst.M_Red_Inst")
  (`KismetSystemLibrary.Delay` 2.0)
  (`self.Disable`))

(event `EmergencyLights`
  (`PrimitiveComponent.SetMaterial` (`self.StaticMeshComponent`) 1 "/Game/Materials/M_Red_Inst.M_Red_Inst")
  (`LightComponent.SetLightColor` (`self.PointLight`) (struct :`R` 0.541667 :`A` 1.0) true)
  (`LightComponent.SetIntensity` (`self.PointLight`) (`self.New Intensity`))
  (goto _label))

(fn `UserConstructionScript`)