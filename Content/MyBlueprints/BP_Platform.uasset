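; BP_Platform is a moving platform that shuttles between two points, either from the start or once activated.
; BeginPlay snaps it to Point1, then starts the loop if Activate is set, otherwise turns the edge glow red.
; The ActivatePlatform dispatcher fires Active, which turns the glow green and starts the loop.
; MoveComponentTo and a FlipFlop alternate the direction, with a delay only after reaching Point2.
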(event `self.ReceiveBeginPlay`
  (bind _ease_in (`self.Ease In`))
  (bind _ease_in_2 (`self.Ease In`))
  (add `self.ActivatePlatform` (delegate `Active`))
  (`SceneComponent.K2_SetWorldLocation` (`self.Platform`) (`SceneComponent.K2_GetComponentLocation` (`self.Point1`)) false false)
  (if (`self.Activate`)
    (`KismetSystemLibrary.MoveComponentTo` (`self.Platform`) (`SceneComponent.RelativeLocation` (`self.Point2`)) (struct) _ease_in _ease_in (`self.Move Time`) :!label _label)
    (`KismetSystemLibrary.Delay` (`self.Pause Time`))
    (`/Engine/EditorBlueprintResources/StandardMacros.FlipFlop` :!label _label_2
      (:`A`
        (`KismetSystemLibrary.MoveComponentTo` (`self.Platform`) (`SceneComponent.RelativeLocation` (`self.Point1`)) (struct) _ease_in_2 _ease_in_2 (`self.Move Time`))
        (goto _label_2))
      (:`B`
        (goto _label)))
    (else
      (`PrimitiveComponent.SetMaterial` (`self.Edge Glow`) 0 "/Game/Materials/M_Red_Inst.M_Red_Inst"))))

(event `Active`
  (`PrimitiveComponent.SetMaterial` (`self.Edge Glow`) 0 "/Game/Materials/M_Green_Inst.M_Green_Inst")
  (goto _label))

(fn `UserConstructionScript`)