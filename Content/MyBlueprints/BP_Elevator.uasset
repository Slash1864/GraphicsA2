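; BP_Elevator is an elevator platform that unlocks and turns green once four puzzle completions are counted.
; When active, overlapping its hitbox moves the cylinder toward Point2, and leaving the hitbox moves it back toward Point1 without checking the active state.
; Event dispatchers drive activation and puzzle counting, and stop the opposing MoveComponentTo whenever the direction changes.
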(event `self.ReceiveBeginPlay`
  (add `self.StopUpwardsMovement` (delegate `EndUpwardsMovement`))
  (add `self.StopDownwardsMovement` (delegate `EndDownwardsMovement`))
  (add `self.ActivatePlatform` (delegate `Activate`))
  (add `self.PuzzleComplete` (delegate `PuzzleCompleted`)))

(event `EndUpwardsMovement`
  (goto _label :!via `Stop`))

(event `EndDownwardsMovement`
  (goto _label_2 :!via `Stop`))

(event `PuzzleCompleted`
  (set `self.NumberOfCompletedPuzzles` (+ (`self.NumberOfCompletedPuzzles`) 1))
  (if (== (`self.NumberOfCompletedPuzzles`) 4)
    (`self.ActivatePlatform`)))

(event `self.Hitbox.OnComponentBeginOverlap`
  (params (OverlappedComponent :type "PrimitiveComponent Object Reference") (OtherActor :type "Actor Object Reference") (OtherComp :type "PrimitiveComponent Object Reference") (OtherBodyIndex :type Integer) (bFromSweep :type Boolean) (SweepResult :type "HitResult Structure (by ref)"))
  (if (`self.Active`)
    (`self.StopDownwardsMovement`)
    (`KismetSystemLibrary.MoveComponentTo` (`self.Cylinder`) (`SceneComponent.RelativeLocation` (`self.Point2`)) (struct) false false (`self.Move Time`) :!label _label)))

(event `Activate`
  (set `self.Active` true)
  (`PrimitiveComponent.SetMaterial` (`self.Cylinder`) 0 "/Game/Materials/M_Green_Inst.M_Green_Inst"))

(event `self.Hitbox.OnComponentEndOverlap`
  (params (OverlappedComponent :type "PrimitiveComponent Object Reference") (OtherActor :type "Actor Object Reference") (OtherComp :type "PrimitiveComponent Object Reference") (OtherBodyIndex :type Integer))
  (`self.StopUpwardsMovement`)
  (`KismetSystemLibrary.MoveComponentTo` (`self.Cylinder`) (`SceneComponent.RelativeLocation` (`self.Point1`)) (struct) false false (`self.Move Time`) :!label _label_2))

(fn `UserConstructionScript`)