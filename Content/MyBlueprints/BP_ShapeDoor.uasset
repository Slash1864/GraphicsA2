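; BP_ShapeDoor is a puzzle door that opens when its shape buttons are pressed in the correct order.
; On BeginPlay it binds to dispatchers for a new press, a wrong order and a correct order.
; Each press increments a counter, and a wrong order calls WrongOrder on all four buttons.
; A correct order moves the Cylinder component to Point2's relative location over MoveTime.
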(event `self.ReceiveBeginPlay`
  (add `self.NewButtonPushed` (delegate `ButtonPushed`))
  (add `self.IncorrectOrder` (delegate `IncorrectButton`))
  (add `self.CorrectOrder` (delegate `CorrectButtonOrder`)))

(event `CorrectButtonOrder`
  (`KismetSystemLibrary.MoveComponentTo` (`self.Cylinder`) (`SceneComponent.RelativeLocation` (`self.Point2`)) (struct) false false (`self.Move Time`)))

(event `ButtonPushed`
  (set `self.ButtonsPressed` (+ (`self.ButtonsPressed`) 1)))

(event `IncorrectButton`
  (`/Game/MyBlueprints/BP_ShapeButton.Wrong Order` (`self.Button1`))
  (`/Game/MyBlueprints/BP_ShapeButton.Wrong Order` (`self.Button2`))
  (`/Game/MyBlueprints/BP_ShapeButton.Wrong Order` (`self.Button3`))
  (`/Game/MyBlueprints/BP_ShapeButton.Wrong Order` (`self.Button4`)))

(fn `UserConstructionScript`)