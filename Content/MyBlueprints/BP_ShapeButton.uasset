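; BP_ShapeButton is a clickable puzzle button that must be pressed in sequence with others to satisfy a linked ShapeDoor.
; A click passes a DoOnce gate, turns the cube green and fires CheckOrder, which updates the door's press count and compares it to the button's Order.
; On the fourth press the door reports success or failure and resets after failure.
; The bound WrongOrder event turns the cube red and re-arms the gate.
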(event `self.ReceiveBeginPlay`
  (add `self.CheckOrder` (delegate `Check`))
  (add `self.Wrong Order` (delegate `Wrong`)))

(event `Wrong`
  (`PrimitiveComponent.SetMaterial` (`self.Cube`) 0 "/Game/Materials/M_Red_Inst.M_Red_Inst")
  (goto _label :!via `Reset`))

(event `Check`
  (`/Game/MyBlueprints/BP_ShapeDoor.NewButtonPushed` (`self.ShapeDoor`))
  (set `self.ButtonsPushed` (`/Game/MyBlueprints/BP_ShapeDoor.ButtonsPressed` (`self.ShapeDoor`)))
  (if (not (== (`self.ButtonsPushed`) (`self.Order`)))
    (set `/Game/MyBlueprints/BP_ShapeDoor.Ordered` false (`self.ShapeDoor`)))
  (if (== 4 (`self.ButtonsPushed`))
    (if (`/Game/MyBlueprints/BP_ShapeDoor.Ordered` (`self.ShapeDoor`))
      (`/Game/MyBlueprints/BP_ShapeDoor.CorrectButtonOrder` (`self.ShapeDoor`))
      (else
        (`/Game/MyBlueprints/BP_ShapeDoor.IncorrectOrder` (`self.ShapeDoor`))
        (set `/Game/MyBlueprints/BP_ShapeDoor.ButtonsPressed` 0 (`self.ShapeDoor`))
        (set `/Game/MyBlueprints/BP_ShapeDoor.Ordered` true (`self.ShapeDoor`))))))

(event `self.ReceiveActorOnClicked`
  (params (ButtonPressed :type "Key Structure"))
  (`/Engine/EditorBlueprintResources/StandardMacros.DoOnce` false :!label _label
    (:`Completed`
      (`PrimitiveComponent.SetMaterial` (`self.Cube`) 0 "/Game/Materials/M_Green_Inst.M_Green_Inst")
      (`self.CheckOrder`))))

(fn `UserConstructionScript`)