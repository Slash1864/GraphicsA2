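; BP_BoxPressurePlate is a pressure plate that a BP_MoveableBox triggers to open a door and set off a scripted level sequence.
; Pressing turns the glow green, opens the door and moves anchors, then after a delay spawns moving master fields, explodes lights, starts smoke, destroys referenced actors and recolours a wall.
; Unless StayActivated, removing the box turns it red, closes the door and re-arms the press; this release is itself a never-reset DoOnce.
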(event `self.ReceiveBeginPlay`)

(event `self.Box.OnComponentBeginOverlap`
  (params (OverlappedComponent :type "PrimitiveComponent Object Reference") (OtherActor :type "Actor Object Reference") (OtherComp :type "PrimitiveComponent Object Reference") (OtherBodyIndex :type Integer) (bFromSweep :type Boolean) (SweepResult :type "HitResult Structure (by ref)"))
  (cast `/Game/MyBlueprints/BP_MoveableBox` OtherActor)
  (`/Engine/EditorBlueprintResources/StandardMacros.DoOnce` false :!label _label
    (:`Completed`
      (`PrimitiveComponent.SetMaterial` (`self.Glow`) 0 "/Game/Materials/M_Green_Inst.M_Green_Inst")
      (set `self.Activate` true)
      (`/Game/MyBlueprints/BP_PuzzleDoor.Open` (`self.DoorRef`))
      (`/Game/MyBlueprints/BP_MovingAnchor.Move` (`self.Anchor1`))
      (`/Game/MyBlueprints/BP_MovingAnchor.Move` (`self.Anchor2`))
      (`KismetSystemLibrary.Delay` 1.0)
      (`|SpawnActorFromClass` "/Game/MyBlueprints/BP_MovingMasterField.BP_MovingMasterField_C" (`self.SpawnTransform1`) "Undefined" "MultiplyWithRoot" null null)
      (`|SpawnActorFromClass` "/Game/MyBlueprints/BP_MovingMasterField.BP_MovingMasterField_C" (`self.SpawnTransform2`) "Undefined" "MultiplyWithRoot" null null)
      (`/Game/MyBlueprints/BP_Light.Explosion` (`self.Light1`))
      (`/Game/MyBlueprints/BP_Light.Explosion` (`self.Light2`))
      (`/Game/MyBlueprints/BP_Light.Explosion` (`self.Light3`))
      (`/Game/MyBlueprints/BP_Light.Explosion` (`self.Light4`))
      (`/Game/MyBlueprints/BP_Light.Explosion` (`self.Light5`))
      (`/Game/MyBlueprints/BP_Light.Explosion` (`self.Light6`))
      (`/Game/MyBlueprints/BP_Light.Explosion` (`self.Light7`))
      (`/Game/MyBlueprints/BP_Light.Explosion` (`self.Light8`))
      (`/Game/MyBlueprints/BP_Light.Explosion` (`self.Light9`))
      (`/Game/MyBlueprints/BP_Light.Explosion` (`self.Light10`))
      (`/Game/MyBlueprints/BP_Light.Explosion` (`self.Light11`))
      (`/Game/MyBlueprints/BP_Light.Explosion` (`self.Light12`))
      (`/Game/MyBlueprints/BP_Light.Explosion` (`self.Light13`))
      (`/Game/MyBlueprints/BP_Light.Explosion` (`self.Light14`))
      (`/Game/MyBlueprints/BP_Light.Explosion` (`self.Light15`))
      (`/Game/MyBlueprints/NS_SmokeEmitter2_Blueprint.Smoke` (`self.Smoke1`))
      (`/Game/MyBlueprints/NS_SmokeEmitter2_Blueprint.Smoke` (`self.Smoke2`))
      (`/Game/MyBlueprints/NS_SmokeEmitter2_Blueprint.Smoke` (`self.Smoke3`))
      (`/Game/MyBlueprints/NS_SmokeEmitter2_Blueprint.Smoke` (`self.Smoke4`))
      (`/Game/MyBlueprints/NS_SmokeEmitter2_Blueprint.Smoke` (`self.Smoke5`))
      (`/Game/MyBlueprints/NS_SmokeEmitter2_Blueprint.Smoke` (`self.Smoke6`))
      (`/Game/MyBlueprints/NS_SmokeEmitter2_Blueprint.Smoke` (`self.Smoke7`))
      (`/Game/MyBlueprints/NS_SmokeEmitter2_Blueprint.Smoke` (`self.Smoke8`))
      (`self.K2_DestroyActor` (`self.Sphere`))
      (`self.K2_DestroyActor` (`self.Sphere2`))
      (`self.K2_DestroyActor` (`self.PlasmaSphere`))
      (`self.K2_DestroyActor` (`self.SlidingDoor1`))
      (`self.K2_DestroyActor` (`self.SlidingDoor2`))
      (`self.K2_DestroyActor` (`self.SlidingDoor3`))
      (`self.K2_DestroyActor` (`self.SlidingDoor4`))
      (`self.K2_DestroyActor` (`self.SlidingDoor5`))
      (`self.K2_DestroyActor` (`self.SlidingDoor6`))
      (`self.K2_DestroyActor` (`self.SlidingDoor7`))
      (`self.K2_DestroyActor` (`self.SlidingDoor8`))
      (`/Game/MyBlueprints/BP_WallColour.ColourChange` (`self.WallColour`)))))

(event `self.Box.OnComponentEndOverlap`
  (params (OverlappedComponent :type "PrimitiveComponent Object Reference") (OtherActor :type "Actor Object Reference") (OtherComp :type "PrimitiveComponent Object Reference") (OtherBodyIndex :type Integer))
  (cast `/Game/MyBlueprints/BP_MoveableBox` OtherActor)
  (if (not (`self.StayActivated`))
    (`/Engine/EditorBlueprintResources/StandardMacros.DoOnce` false
      (:`Completed`
        (`PrimitiveComponent.SetMaterial` (`self.Glow`) 0 "/Game/Materials/M_Red_Inst.M_Red_Inst")
        (set `self.Activate` false)
        (`/Game/MyBlueprints/BP_PuzzleDoor.Close` (`self.DoorRef`))
        (goto _label :!via `Reset`)))))

(fn `UserConstructionScript`)