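; BP_SlidingDoor is a two-panel vertical sliding door that opens on a bound event and closes when its trigger box is overlapped.
; Cube and Cube1 slide between top and bottom marker components using MoveComponentTo over a shared MoveTime.
; On BeginPlay it binds OpenDoor to the open event and, if FrontDoor is set, immediately runs the closing move.
; Any overlap with Box closes the door, with no actor filtering.
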(event `self.ReceiveBeginPlay`
  (add `self.OpenSlidingDoor` (delegate `OpenDoor`))
  (if (`self.FrontDoor`)
    (`KismetSystemLibrary.MoveComponentTo` (`self.Cube`) (`SceneComponent.RelativeLocation` (`self.TopDoorBottom`)) (struct) false false (`self.MoveTime`))
    (`KismetSystemLibrary.MoveComponentTo` (`self.Cube1`) (`SceneComponent.RelativeLocation` (`self.BottomDoorTop`)) (struct) false false (`self.MoveTime`))))

(event `OpenDoor`
  (`KismetSystemLibrary.MoveComponentTo` (`self.Cube`) (`SceneComponent.RelativeLocation` (`self.TopDoorTop`)) (struct) false false (`self.MoveTime`))
  (`KismetSystemLibrary.MoveComponentTo` (`self.Cube1`) (`SceneComponent.RelativeLocation` (`self.BottomDoorBottom`)) (struct) false false (`self.MoveTime`)))

(event `self.Box.OnComponentBeginOverlap`
  (params (OverlappedComponent :type "PrimitiveComponent Object Reference") (OtherActor :type "Actor Object Reference") (OtherComp :type "PrimitiveComponent Object Reference") (OtherBodyIndex :type Integer) (bFromSweep :type Boolean) (SweepResult :type "HitResult Structure (by ref)"))
  (`KismetSystemLibrary.MoveComponentTo` (`self.Cube`) (`SceneComponent.RelativeLocation` (`self.TopDoorBottom`)) (struct) false false (`self.MoveTime`))
  (`KismetSystemLibrary.MoveComponentTo` (`self.Cube1`) (`SceneComponent.RelativeLocation` (`self.BottomDoorTop`)) (struct) false false (`self.MoveTime`)))

(fn `UserConstructionScript`)