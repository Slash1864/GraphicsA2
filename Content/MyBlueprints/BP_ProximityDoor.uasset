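; Proximity door that slides its Cylinder to Point2 when something overlaps the Hitbox and back to Point1 when the overlap ends.
; Two Move Component To nodes handle the upward and downward motion over MoveTime, in relative space.
; Event dispatchers bound on BeginPlay stop the opposite move before each new one starts, so the door can reverse mid-travel.
; Overlaps are not filtered by actor or counted.
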(event `self.ReceiveBeginPlay`
  (add `self.StopUpwardsMovement` (delegate `EndUpwardsMovement`))
  (add `self.StopDownwardsMovement` (delegate `EndDownwardsMovement`)))

(event `EndUpwardsMovement`
  (goto _label :!via `Stop`))

(event `EndDownwardsMovement`
  (goto _label_2 :!via `Stop`))

(event `self.Hitbox.OnComponentBeginOverlap`
  (params (OverlappedComponent :type "PrimitiveComponent Object Reference") (OtherActor :type "Actor Object Reference") (OtherComp :type "PrimitiveComponent Object Reference") (OtherBodyIndex :type Integer) (bFromSweep :type Boolean) (SweepResult :type "HitResult Structure (by ref)"))
  (`self.StopDownwardsMovement`)
  (`KismetSystemLibrary.MoveComponentTo` (`self.Cylinder`) (`SceneComponent.RelativeLocation` (`self.Point2`)) (struct) false false (`self.Move Time`) :!label _label))

(event `self.Hitbox.OnComponentEndOverlap`
  (params (OverlappedComponent :type "PrimitiveComponent Object Reference") (OtherActor :type "Actor Object Reference") (OtherComp :type "PrimitiveComponent Object Reference") (OtherBodyIndex :type Integer))
  (`self.StopUpwardsMovement`)
  (`KismetSystemLibrary.MoveComponentTo` (`self.Cylinder`) (`SceneComponent.RelativeLocation` (`self.Point1`)) (struct) false false (`self.Move Time`) :!label _label_2))

(fn `UserConstructionScript`)